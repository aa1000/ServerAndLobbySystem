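; Lobby player controller that creates and shows the lobby menu widget when the player enters the lobby.
; On BeginPlay it creates the LobbyMenu with references to itself and the game instance, adds it to the viewport and stores it on BP_NWGameInstance.
; ChatMessage and UpdateUMGPlayerList events forward incoming chat and the server-sent player info array to the widget for display.
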(event `self.ReceiveBeginPlay`
  ;[1 1 1] create the lobby and view it as soon as the player gets in
  (`parent.ReceiveBeginPlay`)
  (bind _asbp_nwgame_instance (cast `/Game/Network/Blueprints/BP_NWGameInstance` (`GameplayStatics.GetGameInstance`)) ; Should always work since we are in a game
    (:`then`
      _)
    (:`CastFailed`
      _))
  (bind _returnvalue (`|CreateWidget` "/Game/Lobby/UI/LobbyMenu.LobbyMenu_C" self self _asbp_nwgame_instance))
  (bind _output_get (set `self.LobbyWidget` _returnvalue))
  (`UserWidget.AddToViewport` _output_get 0)
  (set `/Game/Network/Blueprints/BP_NWGameInstance.LobbyMenuWidget` _output_get _asbp_nwgame_instance))

(event `self.ReceiveChatMessage`
  (params (ChatMessage :type "Text (by ref)"))
  ;[1 1 1] pass the incoming chat message to UMG
  (`/Game/Lobby/UI/LobbyMenu.ReceiveChatMessage` (`self.LobbyWidget`) ChatMessage))

(event `self.UpdateUMGPlayerList`
  (params (PlayerInfoArray :type "Array of LobbyPlayerInfo Structure (by ref)"))
  ;[1 1 1] passes in the array ther server sent to UMG so the player can see it
  (`/Game/Lobby/UI/LobbyMenu.UpdatePlayerList` (`self.LobbyWidget`) PlayerInfoArray))

(fn `UserConstructionScript`)