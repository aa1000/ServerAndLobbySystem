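; Network game instance that owns the main menu, server menu and error message UI for multiplayer.
; Show events lazily create each widget, cache it and re-add it to the viewport on later calls, updating the error text as needed.
; Completion events relay session search results to the server menu and Steam friend lists, supplied from code, to the lobby menu if it is valid.
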(event `ShowMainMenu`
  ;[1 1 1] called to show the MainMenu, if the main menu was created before, just show it, if not then create it, save it in a variable and show it
  (`/Engine/EditorBlueprintResources/StandardMacros.IsValid` (`self.MainMenuWidget`)
    (:`Is Valid`
      (`UserWidget.AddToViewport` (`self.MainMenuWidget`) 0))
    (:`Is Not Valid`
      (bind _returnvalue (`|CreateWidget` "/Game/MainMenu/UI/MainMenu.MainMenu_C" (`GameplayStatics.GetPlayerController` 0) self (`self.MinServerNameLength`) (`self.MaxServerNameLength`) 50))
      (bind _output_get (set `self.MainMenuWidget` _returnvalue))
      (`UserWidget.AddToViewport` _output_get 0))))

(event `self.ShowErrorMessageUMG`
  (params (ErrorMessage :type "Text (by ref)"))
  (bind _errormessagewidget (`self.ErrorMessageWidget`))
  (`/Engine/EditorBlueprintResources/StandardMacros.IsValid` (`self.ErrorMessageWidget`)
    (:`Is Valid`
      ;[1 1 1] if the widget was created already, change the error text and display it
      (set `/Game/Network/UI/OkErrorMessageWidget.ErrorText` ErrorMessage _errormessagewidget)
      (`UserWidget.AddToViewport` _errormessagewidget 0))
    (:`Is Not Valid`
      ;[1 1 1] if the widget was not created before, create it, set the error text and then show it to the player
      (bind _returnvalue (`|CreateWidget` "/Game/Network/UI/OkErrorMessageWidget.OkErrorMessageWidget_C" (`GameplayStatics.GetPlayerController` 0) ErrorMessage))
      (bind _output_get (set `self.ErrorMessageWidget` _returnvalue))
      (`UserWidget.AddToViewport` _output_get 0))))

(event `ShowServerMenu`
  ;[1 1 1] called to show the ServerMenu, if the server menu was created before, just show it, if not then create it, save it in a variable and show it
  (`/Engine/EditorBlueprintResources/StandardMacros.IsValid` (`self.ServerMenuWidget`)
    (:`Is Valid`
      (`UserWidget.AddToViewport` (`self.ServerMenuWidget`) 0))
    (:`Is Not Valid`
      (bind _returnvalue (`|CreateWidget` "/Game/Network/UI/ServerMenu.ServerMenu_C" (`GameplayStatics.GetPlayerController` 0) self))
      (bind _output_get (set `self.ServerMenuWidget` _returnvalue))
      (`UserWidget.AddToViewport` _output_get 0))))

(event `self.OnFoundSessionsCompleteUMG`
  (params (CustomSessionResults :type "Array of CustomBlueprintSessionResult Structure (by ref)"))
  ;[1 1 1] call the ServerMenu UMG and pass the array of Session Results when yhe session finding is over
  (`/Game/Network/UI/ServerMenu.SessionSearchCompleated` (`self.ServerMenuWidget`) CustomSessionResults))

(event `self.OnGetSteamFriendRequestCompleteUMG`
  (params (BPFriendsLists :type "Array of SteamFriendInfo Structure (by ref)"))
  (bind _lobbymenuwidget (`self.LobbyMenuWidget`))
  ;[1 1 1] called from code when it finishes getting the friendlist and passes it to blueprint
  (`/Engine/EditorBlueprintResources/StandardMacros.IsValid` _lobbymenuwidget
    (:`Is Valid`
      (`/Game/Lobby/UI/LobbyMenu.GetSteamFriendRequestCompleted` _lobbymenuwidget BPFriendsLists))))