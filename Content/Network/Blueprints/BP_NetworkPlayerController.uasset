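; BP_NetworkPlayerController is a player controller for the network game that handles sign interaction UI and quitting.
; On BeginPlay it clears all widgets and caches the BP_NWGameInstance.
; WidgetonUse creates a NetworkSignWidget owned by this controller, passes it the first BP_NetworkSign found in the world, and adds it to the viewport.
; The Escape key quits the game.
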(event `self.ReceiveBeginPlay`
  (`WidgetLayoutLibrary.RemoveAllWidgets`)
  (bind _asbp_nwgame_instance (cast `/Game/Network/Blueprints/BP_NWGameInstance` (`GameplayStatics.GetGameInstance`)))
  (set `self.NetworkGameInstance` _asbp_nwgame_instance))

(event `Key|Escape`
  (params (Key :type "Key Structure" :default "AnyKey"))
  (:`Pressed`
    (`KismetSystemLibrary.QuitGame` self "Quit")))

(event `self.WidgetOnUse`
  (params (PC :type "PlayerController Object Reference"))
  (bind _outactors (`GameplayStatics.GetAllActorsOfClass` "/Game/Items/Blueprints/BP_NetworkSign.BP_NetworkSign_C"))
  (bind _returnvalue (`|CreateWidget` "/Game/Items/Ui/NetworkSignWidget.NetworkSignWidget_C" self (`KismetArrayLibrary.Array_Get` _outactors) self))
  (`UserWidget.AddToViewport` _returnvalue 0))

(fn `UserConstructionScript`)